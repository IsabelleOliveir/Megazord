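; Playable pinball minigame actor that the player enters and exits through Interagir, which switches the view, input lock, inventory visibility and playing flag.
; Tick reads the ThirdPersonCharacter's input flags to drive timelines for both flippers, the launch piston and tilt shake.
; These timelines are chained, each next check running from the previous one's Update.
; Balls spawn on BeginPlay and respawn with alternating color after hitting EndGame.
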(event `self.ReceiveBeginPlay`
  ;[0.0356 0 0.001214 0.3608] Referência do Jogador
  (bind _asthird_person_character (cast `/Game/HomeWork/Characters/Luffy/ThirdPersonCharacter` (`GameplayStatics.GetPlayerCharacter` 0)))
  (set `self.Ref Jogador` _asthird_person_character)
  ;[0.0356 0 0.001214 0.3608] Pega a rotação mínima do Flipper
  (set `self.RotMin_FlipperDireito` (`SceneComponent.RelativeRotation` (`self.PB_FlipperDireito`)))
  (set `self.RotMin_FlipperEsquerdo` (`SceneComponent.RelativeRotation` (`self.PB_FlipperEsquerdo`)))
  ;[0.0356 0 0.001214 0.3608] Spawna a primeira bolinha
  (bind _returnvalue (`|SpawnActorFromClass` "/Game/HomeWork/Maps/Map/Pinball/BP/BP_Bolinha.BP_Bolinha_C" (`KismetMathLibrary.MakeTransform` (`SceneComponent.K2_GetComponentLocation` (`self.SpawnBolinha`)) (struct) (0.07 0.07 0.07)) "Undefined" "OverrideRootScale" null "NewEnumerator1" null))
  (set `self.Bolinha` _returnvalue)
  ;[0.0356 0 0.001214 0.3608] Pega a rotação do pinball (para o tilt)
  (set `self.RotPinball` (`SceneComponent.RelativeRotation` (`self.PB_EstruturaPrincipal`))))

(event `self.PB_Pistão.OnComponentHit`
  (params (HitComponent :type "PrimitiveComponent Object Reference") (OtherActor :type "Actor Object Reference") (OtherComp :type "PrimitiveComponent Object Reference") (NormalImpulse :type "Vector Structure") (Hit :type "HitResult Structure (by ref)"))
  ;[0.0625 0 0.0179] Codigos que podem ajudar eventualmente
  ;;[0 0 0 0.3608] (Inativo) Impulso no pistão de lançamento (pq tava fraco)
)

(event `self.ReceiveTick`
  (params (DeltaSeconds :type "Float (single-precision)"))
  (bind _returnvalue (`KismetMathLibrary.Conv_RotatorToVector` (`self.RotPinball`)))
  ;[0.1354 0.111 0.04514] Flipper Esquerdo
  (if (`/Game/HomeWork/Characters/Luffy/ThirdPersonCharacter.PB_PressLeft` (`self.Ref Jogador`))
    (bind (_direction `_tempo_de_transição`) (`Timeline|Timeline_Flipper_Esquerdo` :!label _label)
      (:`Update`
        (`SceneComponent.K2_SetRelativeRotation` (`self.PB_FlipperEsquerdo`) (`KismetMathLibrary.RLerp` (`self.RotMin_FlipperEsquerdo`) (`self.RotMax_FlipperEsquerdo`) `_tempo_de_transição`) false false)
        ;[0.08519 0.05867 0.1094] Flipper Direito
        (if (`/Game/HomeWork/Characters/Luffy/ThirdPersonCharacter.PB_PressRight` (`self.Ref Jogador`))
          (bind (_direction_2 `_tempo_de_transição_2`) (`Timeline|Timeline Flipper Direito` :!label _label_2)
            (:`Update`
              (`SceneComponent.K2_SetRelativeRotation` (`self.PB_FlipperDireito`) (`KismetMathLibrary.RLerp` (`self.RotMin_FlipperDireito`) (`self.RotMax_FlipperDireito`) `_tempo_de_transição_2`) false false)
              ;[0 0 0 0.3608] Lançamento da Bolinha
              (if (`/Game/HomeWork/Characters/Luffy/ThirdPersonCharacter.PB_PressForce` (`self.Ref Jogador`))
                (bind (_direction_3 `_lançamento`) (`Timeline|Timeline Lançamento da Bolinha` :!label _label_3)
                  (:`Update`
                    (set `self.Lançamento` `_lançamento`)
                    (if (`self.IsLauch`)
                      (set `self.Lançamento` (`KismetMathLibrary.FClamp` (* (`self.Lançamento`) 0.0001))))
                    (`SceneComponent.K2_SetRelativeLocation` (`self.PB_Pistão`) (`KismetMathLibrary.VLerp` (855.0 1895.0 28.0) (855.0 2090.0 28.0) (`self.Lançamento`)) false false)
                    ;[0 0 0 0.3608] Tilt
                    (if (`/Game/HomeWork/Characters/Luffy/ThirdPersonCharacter.Tilt` (`self.Ref Jogador`))
                      (bind (_direction_4 `_tremulação`) (`Timeline|Timeline_Tilt` :!via `PlayFromStart` :!label _label_4)
                        (:`Update`
                          (`SceneComponent.K2_SetRelativeRotation` (`self.PB_EstruturaPrincipal`) (`KismetMathLibrary.RLerp` (`KismetMathLibrary.Conv_VectorToRotator` (+ _returnvalue (5.0 0.0 0.0))) (`KismetMathLibrary.Conv_VectorToRotator` (+ _returnvalue (-5.0 0.0 0.0))) `_tremulação`) false false)
                          (`KismetSystemLibrary.Delay` 0.1)
                          (`SceneComponent.K2_SetRelativeRotation` (`self.PB_EstruturaPrincipal`) (`self.RotPinball`) false false)))
                      (else
                        (goto _label_4 :!via `Reverse`))))
                  (:`Finished`
                    (set `self.IsLauch` false)))
                (else
                  (set `self.IsLauch` true)
                  (goto _label_3 :!via `Reverse`)))))
          (else
            (goto _label_2 :!via `Reverse`)))))
    (else
      (goto _label :!via `Reverse`))))

(event `self.EndGame.OnComponentBeginOverlap`
  (params (OverlappedComponent :type "PrimitiveComponent Object Reference") (OtherActor :type "Actor Object Reference") (OtherComp :type "PrimitiveComponent Object Reference") (OtherBodyIndex :type Integer) (bFromSweep :type Boolean) (SweepResult :type "HitResult Structure (by ref)"))
  ;[0 0 0 0.3608] Destroy e Spawn da Bolinha
  ;;[0.04688 0 0 0.3608] Destroi a bolinha assim que ela encosta no EndGame
  (bind _asbp_bolinha (cast `/Game/HomeWork/Maps/Map/Pinball/BP/BP_Bolinha` OtherActor))
  (`self.K2_DestroyActor` _asbp_bolinha)
  ;;[0.000106 0.02456 0.04167 0.3608] Spawna a bolinha depois que ela é destruida
  (`/Engine/EditorBlueprintResources/StandardMacros.FlipFlop`
    (:`A`
      (bind _returnvalue (`|SpawnActorFromClass` "/Game/HomeWork/Maps/Map/Pinball/BP/BP_Bolinha.BP_Bolinha_C" (`KismetMathLibrary.MakeTransform` (`SceneComponent.K2_GetComponentLocation` (`self.SpawnBolinha`)) (struct) (0.07 0.07 0.07)) "Undefined" "OverrideRootScale" null "NewEnumerator0" null))
      (set `self.Bolinha` _returnvalue))
    (:`B`
      (bind _returnvalue_2 (`|SpawnActorFromClass` "/Game/HomeWork/Maps/Map/Pinball/BP/BP_Bolinha.BP_Bolinha_C" (`KismetMathLibrary.MakeTransform` (`SceneComponent.K2_GetComponentLocation` (`self.SpawnBolinha`)) (struct) (0.07 0.07 0.07)) "Undefined" "OverrideRootScale" null "NewEnumerator1" null))
      (set `self.Bolinha` _returnvalue_2))))

(event `/Game/HomeWork/BPI_Interagir.Interagir`
  (bind _returnvalue (`GameplayStatics.GetPlayerController` 0))
  (bind _returnvalue_2 (`GameplayStatics.GetPlayerController` 0))
  ;[0 0 0 0.3608] Faz a câmera mudar para a câmera do minigame
  (`/Engine/EditorBlueprintResources/StandardMacros.FlipFlop`
    (:`A`
      ;;[0.04667 0.04667 0.04667 0.3608] Bloqueia os movimentos do personagem
      (`Controller.SetIgnoreMoveInput` _returnvalue_2 true)
      (`Controller.SetIgnoreLookInput` _returnvalue_2 true)
      (`PlayerController.SetViewTargetWithBlend` _returnvalue_2 self 0.0 "VTBlend_Linear" 0.0 false)
      (`Widget.SetVisibility` (`/Game/HomeWork/Characters/Luffy/ThirdPersonCharacter.Inventario` (`self.Ref Jogador`)) "Hidden")
      ;;[0.04667 0.04667 0.04667 0.3608] Seta que o personagem ESTÁ jogando
      (set `/Game/HomeWork/Characters/Luffy/ThirdPersonCharacter.EstaJogando` true (`self.Ref Jogador`)))
    (:`B`
      ;;[0.04667 0.04667 0.04667 0.3608] Reseta os movimentos do personagem
      (`Controller.ResetIgnoreMoveInput` _returnvalue)
      (`Controller.ResetIgnoreLookInput` _returnvalue)
      (`PlayerController.SetViewTargetWithBlend` _returnvalue (`GameplayStatics.GetPlayerCharacter` 0) 0.0 "VTBlend_Linear" 0.0 false)
      (`Widget.SetVisibility` (`/Game/HomeWork/Characters/Luffy/ThirdPersonCharacter.Inventario` (`self.Ref Jogador`)) "Visible")
      ;;[0.04667 0.04667 0.04667 0.3608] Seta que o personagem NÃO ESTÁ jogando
      (set `/Game/HomeWork/Characters/Luffy/ThirdPersonCharacter.EstaJogando` false (`self.Ref Jogador`)))))

(fn `UserConstructionScript`)