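; BP_Bolinha is the physics ball actor in the Pinball map, available in yellow or purple.
; On BeginPlay, the Cor enum selects the Bolinha component's material and its custom collision object type, giving each color its own collision channel.
; Every tick, it clamps the component's linear velocity to cap the ball's maximum speed.
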(event `self.ReceiveBeginPlay`
  ;[0 0 0 0.3608] Seta material e colisão para cada item do meu Enum
  (switch `/Game/HomeWork/Maps/Map/Pinball/Enum/CorDaBolinha` (`self.Cor`)
    (:`NewEnumerator0`
      (`PrimitiveComponent.SetMaterial` (`self.Bolinha`) 0 "/Game/HomeWork/Maps/MaterialLibrary/MaterialInstances/MI_Amarelo.MI_Amarelo")
      (`PrimitiveComponent.SetCollisionObjectType` (`self.Bolinha`) "ECC_GameTraceChannel1"))
    (:`NewEnumerator1`
      (`PrimitiveComponent.SetMaterial` (`self.Bolinha`) 0 "/Game/HomeWork/Maps/MaterialLibrary/MaterialInstances/MI_Roxo.MI_Roxo")
      (`PrimitiveComponent.SetCollisionObjectType` (`self.Bolinha`) "ECC_GameTraceChannel2"))))

(event `self.ReceiveTick`
  (params (DeltaSeconds :type "Float (single-precision)"))
  ;[0 0 0] Define velocidade máxima para a bolinha
  (bind _returnvalue (`PrimitiveComponent.GetPhysicsLinearVelocity` (`self.Bolinha`) "None"))
  (`PrimitiveComponent.SetPhysicsLinearVelocity` (`self.Bolinha`) (`KismetMathLibrary.ClampVectorSize` _returnvalue 0.0 2000.0) false "None"))

(fn `UserConstructionScript`)